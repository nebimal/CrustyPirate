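; Anim notify state that sets the active window of the player's attack hitbox during an animation.
; On begin, it casts the mesh's owning actor to Blueprint_PlayerCharacter and enables its attack collision box; on end, it disables the box the same way.
; Other owners fail the cast and are ignored.
; The EventGraph holds unconnected duplicates of this logic that never run.
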(fn OnNotifyBegin
  (params (OwningInstance :type Paper%20ZD%20Anim%20Instance%20Object%20Reference))
  (bind _asblueprint_player_character (Utilities|Casting|CastToBlueprint_PlayerCharacter (Class|PaperZDAnimInstance|GetOwningActor OwningInstance)))
  (Class|PlayerCharacter|EnableAttackCollisionBox _asblueprint_player_character true))

(fn OnNotifyEnd
  (params (OwningInstance :type Paper%20ZD%20Anim%20Instance%20Object%20Reference))
  (bind _asblueprint_player_character (Utilities|Casting|CastToBlueprint_PlayerCharacter (Class|PaperZDAnimInstance|GetOwningActor OwningInstance)))
  (Class|PlayerCharacter|EnableAttackCollisionBox _asblueprint_player_character false))